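; BP_Boss is a boss character driven by the BT_Boss behavior tree, which its AI controller starts on BeginPlay.
; PawnSensing passes each seen pawn, along with the player pawn, to DetectPawn, whose logic lives outside these graphs.
; Selection and deselection events show and hide a lock-on widget, so the boss can act as a target.
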(event OnSeePawn(PawnSensing)
  (params (Pawn :type Pawn%20Object%20Reference))
  (Class|BossCharacter|DetectPawn Pawn (Game|Player|GetPlayerPawn 0)))

(event EventBeginPlay
  (AI|RunBehaviorTree (AI|GetAIController self) "/Game/AI/BT_Boss.BT_Boss"))

(event Collision|EventActorBeginOverlap
  (params (OtherActor :type Actor%20Object%20Reference)))

(event EventTick
  (params (DeltaSeconds :type Float%20%28single-precision%29)))

(event EventOnSelected
  (Rendering|SetVisibility (Variables|Default|GetLockonWidget) true false))

(event EventOnDeselected
  (Rendering|SetVisibility (Variables|Default|GetLockonWidget) false false))

(fn ConstructionScript)